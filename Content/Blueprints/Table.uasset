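; Restaurant table actor that displays its number and highlights itself when the waiter carrying a plate is close enough to put food down.
; BeginPlay writes the table number to a text render component.
; Each Tick finds the first WaiterBP; while it holds a plate, a distance check toggles the mesh's custom depth glow and sets WaiterCloseBy.
; Without a plate the glow turns off, but WaiterCloseBy keeps its last value.
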(event EventBeginPlay
  ;[1 1 1] Sets Up Rendertext Table Numbers
  (Rendering|Components|TextRender|SetText (Variables|Default|GetTableNum) (Utilities|Text|ToText(Integer) (Variables|Default|GetNumber))))

(event Collision|EventActorBeginOverlap
  (params (OtherActor :type Actor%20Object%20Reference)))

(event EventTick
  (params (DeltaSeconds :type Float%20%28single-precision%29))
  (bind _table (Variables|Default|GetTable))
  ;[1 1 1] Table Glows When Player Can Put Food Down
  (bind _outactors (Actor|GetAllActorsOfClass "/Game/Blueprints/WaiterBP.WaiterBP_C"))
  (if (Variables|/Game/Blueprints/WaiterBP.WaiterBP_C|GetholdingPlate (Utilities|Array|Get(acopy) _outactors))
    (Rendering|SetRenderCustomDepth _table (<= (Math|Vector|Distance(Vector) (Transformation|GetActorLocation) (Transformation|GetActorLocation (Utilities|Array|Get(acopy) _outactors))) 125.0))
    (if (<= (Math|Vector|Distance(Vector) (Transformation|GetActorLocation) (Transformation|GetActorLocation (Utilities|Array|Get(acopy) _outactors))) 125.0)
      (Variables|Default|SetWaiterCloseBy true)
      (else
        (Variables|Default|SetWaiterCloseBy false)))
    (else
      (Rendering|SetRenderCustomDepth _table false))))

(fn ConstructionScript)