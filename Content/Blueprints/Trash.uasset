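; Trash can actor where the player's waiter can discard a carried order.
; Each tick it checks whether the waiter pawn holds a plate and is within a short range.
; While both hold, the can's custom depth highlights it, and pressing Space calls the waiter's discard-order function.
; Input is polled directly from the player controller on Tick rather than through input events or overlap triggers.
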(event EventBeginPlay)

(event Collision|EventActorBeginOverlap
  (params (OtherActor :type Actor%20Object%20Reference)))

(event EventTick
  (params (DeltaSeconds :type Float%20%28single-precision%29))
  (bind _can (Variables|Default|GetCan))
  (bind _aswaiter_standing_bp (Utilities|Casting|CastToWaiterStandingBP (Game|Player|GetPlayerPawn 0)))
  (if (Variables|/Game/Blueprints/WaiterStandingBP.WaiterStandingBP_C|GetholdingPlate _aswaiter_standing_bp)
    (Rendering|SetRenderCustomDepth _can (<= (Math|Vector|Distance(Vector) (Transformation|GetActorLocation) (Transformation|GetActorLocation _aswaiter_standing_bp)) 125.0))
    (if (<= (Math|Vector|Distance(Vector) (Transformation|GetActorLocation) (Transformation|GetActorLocation _aswaiter_standing_bp)) 125.0)
      (if (Game|Player|WasInputKeyJustPressed (Game|GetPlayerController 0) "SpaceBar")
        (Default|CallDiscardOrder _aswaiter_standing_bp (<= (Math|Vector|Distance(Vector) (Transformation|GetActorLocation) (Transformation|GetActorLocation _aswaiter_standing_bp)) 125.0))))
    (else
      (Rendering|SetRenderCustomDepth _can false))))

(fn ConstructionScript)