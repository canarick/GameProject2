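; Plate actor for a waiter game, representing a dish that the waiter can pick up or that sits on a table.
; On BeginPlay, a plate on a table destroys itself after a short timer, while any other sets its name text from the Dish index.
; Each Tick looks up the first WaiterStandingBP and toggles custom depth to make an off-table plate glow when an empty-handed waiter is within range.
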(event Custom|Disappear
  (Actor|DestroyActor))

(event EventBeginPlay
  (if (Variables|Default|GetonTable)
    (Utilities|Time|SetTimerbyEvent (delegate Custom|Disappear) 5.0)
    (else
      (switch int (Variables|Default|GetDish)
        (:0
          (Variables|Default|SetDishString "ratatouille"))
        (:1
          (Variables|Default|SetDishString "soup"))
        (:2
          (Variables|Default|SetDishString "baguette")))
      (Rendering|Components|TextRender|SetText (Variables|Default|GetDishName) (Variables|Default|GetDishString)))))

(event Collision|EventActorBeginOverlap
  (params (OtherActor :type Actor%20Object%20Reference)))

(event EventTick
  (params (DeltaSeconds :type Float%20%28single-precision%29))
  (bind _plate (Variables|Default|GetPlate))
  ;[1 1 1] Plate Glows When Player Can Pick Up
  (bind _outactors (Actor|GetAllActorsOfClass "/Game/Blueprints/WaiterStandingBP.WaiterStandingBP_C"))
  (if (not (Variables|Default|GetonTable))
    (if (Variables|/Game/Blueprints/WaiterStandingBP.WaiterStandingBP_C|GetholdingPlate (Utilities|Array|Get(acopy) _outactors))
      (Rendering|SetRenderCustomDepth _plate false)
      (else
        (Rendering|SetRenderCustomDepth _plate (<= (Math|Vector|Distance(Vector) (Transformation|GetActorLocation) (Transformation|GetActorLocation (Utilities|Array|Get(acopy) _outactors))) 84.0))))))

(fn ConstructionScript)