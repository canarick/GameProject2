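; MouseOrderBP is an actor for a timed dish order that destroys itself when its time runs out.
; On BeginPlay, the Dish value selects the order's duration, which seeds TimeLeft and starts a one-shot expiry timer.
; Tick separately counts TimeLeft down and raises the Warning flag in the final seconds, while the timer event handles the actual destruction.
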(event Custom|OrderExpire
  (Actor|DestroyActor))

(event EventBeginPlay
  (switch int (Variables|Default|GetDish)
    (:0
      (bind _output_get (Variables|Default|SetOrderTime 4e+01))
      (Variables|Default|SetTimeLeft _output_get))
    (:1
      (bind _output_get_2 (Variables|Default|SetOrderTime 35.0))
      (Variables|Default|SetTimeLeft _output_get_2))
    (:2
      (bind _output_get_3 (Variables|Default|SetOrderTime 3e+01))
      (Variables|Default|SetTimeLeft _output_get_3)))
  (Utilities|Time|SetTimerbyEvent (delegate Custom|OrderExpire) (Variables|Default|GetOrderTime)))

(event Collision|EventActorBeginOverlap
  (params (OtherActor :type Actor%20Object%20Reference)))

(event EventTick
  (params (DeltaSeconds :type Float%20%28single-precision%29))
  (bind _output_get (Variables|Default|SetTimeLeft (- (Variables|Default|GetTimeLeft) DeltaSeconds)))
  (if (<= _output_get 1e+01)
    (Variables|Default|SetWarning true)))

(fn ConstructionScript)