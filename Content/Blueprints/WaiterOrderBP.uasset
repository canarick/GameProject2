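; WaiterOrderBP is a timed waiter order for a table, removed when completed or expired.
; On BeginPlay, Dish sets the time limit, starts an expiry timer and binds completion to the first WaiterStandingBP, matching table and dish.
; Tick counts down and flags a warning near expiry.
; Expiry increments OrdersMissed on the Global actor, except table 11, which calls CallMouseWon, then destroys the order.
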(event Custom|OrderCompleted
  (params (Dish :type Integer) (TableNum :type Integer))
  ;[1 1 1] Check if order completed
  (if (== TableNum (Variables|Default|GetTable))
    (if (== Dish (Variables|Default|GetDish))
      (Actor|DestroyActor))))

(event Custom|OrderExpire
  ;[1 1 1] Timer for order expiration
  (bind _outactors (Actor|GetAllActorsOfClass "/Game/Global.Global_C"))
  (if (== 11 (Variables|Default|GetTable))
    (Default|CallMouseWon (Utilities|Array|Get(acopy) _outactors))
    (else
      (Variables|/Game/Global.Global_C|SetOrdersMissed (Utilities|Array|Get(acopy) _outactors) (+ (Variables|/Game/Global.Global_C|GetOrdersMissed (Utilities|Array|Get(acopy) _outactors)) 1))))
  (Actor|DestroyActor))

(event EventBeginPlay
  ;[1 1 1] Initialize Order
  (switch int (Variables|Default|GetDish)
    (:0
      (bind _output_get (Variables|Default|SetOrderTime 45.0))
      (Variables|Default|SetTimeLeft _output_get))
    (:1
      (bind _output_get_2 (Variables|Default|SetOrderTime 3e+01))
      (Variables|Default|SetTimeLeft _output_get_2))
    (:2
      (bind _output_get_3 (Variables|Default|SetOrderTime 25.0))
      (Variables|Default|SetTimeLeft _output_get_3)))
  ;[1 1 1] Timer for order expiration
  (Utilities|Time|SetTimerbyEvent (delegate Custom|OrderExpire) (Variables|Default|GetOrderTime))
  ;[1 1 1] Check if order completed
  (bind _outactors (Actor|GetAllActorsOfClass "/Game/Blueprints/WaiterStandingBP.WaiterStandingBP_C"))
  (EventDispatchers|BindEventtoRemoveOrder (Utilities|Array|Get(acopy) _outactors) (delegate Custom|OrderCompleted)))

(event Collision|EventActorBeginOverlap
  (params (OtherActor :type Actor%20Object%20Reference)))

(event EventTick
  (params (DeltaSeconds :type Float%20%28single-precision%29))
  ;[1 1 1] Update time left
  (bind _output_get (Variables|Default|SetTimeLeft (- (Variables|Default|GetTimeLeft) DeltaSeconds)))
  (if (<= _output_get 1e+01)
    (Variables|Default|SetWarning true)))

(fn ConstructionScript)