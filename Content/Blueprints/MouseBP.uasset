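; MouseBP is the player-controlled mouse that collects and delivers dish orders in a game against a waiter.
; W and A/D move and turn it, passing each change to ROC events that apply the same transform.
; Tick outlines it via custom depth near a broom-holding waiter and handles Space at fixed spots: order drop-off, or winning once enough are fulfilled.
; A bound reset event returns it to its start and clears physics velocity.
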(event Custom|ResetEvent
  (bind _mousecollider (Variables|Default|GetMouseCollider))
  ;[1 1 1] Mouse Reset Event
  (Transformation|SetActorLocationAndRotation "-260.000000,-560.000000,0.000000" "0, 0, 0")
  (Class|PrimitiveComponent|SetAllPhysicsLinearVelocity _mousecollider "0, 0, 0" false)
  (Class|PrimitiveComponent|SetPhysicsAngularVelocityinDegrees _mousecollider "0, 0, 0" false "None"))

(event Custom|ROCLocation
  (params (NewParam :type Vector))
  (Transformation|AddWorldOffset (Variables|Default|GetMouseCollider) NewParam false false))

(event Custom|ROCRotation
  (params (NewParam :type Rotator))
  (Transformation|SetActorRotation NewParam))

(event EventBeginPlay
  ;[1 1 1] Keep reference to waiter
  (bind _outactors (Actor|GetAllActorsOfClass "/Game/Blueprints/WaiterStandingBP.WaiterStandingBP_C"))
  (Variables|Default|SetWaiter (Utilities|Array|Get(acopy) _outactors))
  ;[1 1 1] Mouse Reset Event
  (EventDispatchers|BindEventtoResetMouse (delegate Custom|ResetEvent)))

(event Collision|EventActorBeginOverlap
  (params (OtherActor :type Actor%20Object%20Reference)))

(event EventTick
  (params (DeltaSeconds :type Float%20%28single-precision%29))
  (bind _waiter (Variables|Default|GetWaiter))
  (bind _mousemesh (Variables|Default|GetMouseMesh))
  ;[1 1 1] Glow when in range of waiter hit
  (bind _aswaiter_standing_bp (Utilities|Casting|CastToWaiterStandingBP _waiter))
  (if (Variables|/Game/Blueprints/WaiterStandingBP.WaiterStandingBP_C|GetholdingBroom _aswaiter_standing_bp)
    (if (< (Transformation|GetDistanceTo _waiter) 1e+02)
      (Rendering|SetRenderCustomDepth _mousemesh true)
      (else
        (Rendering|SetRenderCustomDepth _mousemesh false))))
  ;[1 1 1] Drop off Orders
  (Utilities|Casting|CastToMouseBP (Game|Player|GetPlayerPawn 0))
  (if (Game|Player|WasInputKeyJustPressed (Game|GetPlayerController 0) "SpaceBar")
    (if (<= (Math|Vector|Distance(Vector) (Transformation|GetActorLocation) (Math|Vector|MakeVector -2.3e+02 -6.7e+02 0.0)) 1e+02)
      (bind _outactors (Actor|GetAllActorsOfClass "/Game/Blueprints/MouseCollected.MouseCollected_C"))
      (for _array_element _outactors
        (bind _outactors_2 (Actor|GetAllActorsOfClass "/Game/Blueprints/MouseOrderBP.MouseOrderBP_C"))
        (bind _array_element_2 (Utilities|Array|ForEachLoopwithBreak _outactors_2 :!label _label)
          (:LoopBody
            (if (== (Variables|/Game/Blueprints/MouseOrderBP.MouseOrderBP_C|GetDish _array_element_2) (Variables|/Game/Blueprints/MouseCollected.MouseCollected_C|GetDish _array_element))
              (Default|CallDropAll (Variables|/Game/Blueprints/MouseOrderBP.MouseOrderBP_C|GetDish _array_element_2))
              (Actor|DestroyActor _array_element_2)
              (goto _label Break)))
          (:Completed
            (Actor|DestroyActor _array_element))))
      (else
        (bind _outactors_3 (Actor|GetAllActorsOfClass "/Game/Global.Global_C"))
        (if (<= (Math|Vector|Distance(Vector) (Transformation|GetActorLocation) (Math|Vector|MakeVector 2.1e+02 5.7e+02 0.0)) 1.5e+02)
          (if (>= (Variables|/Game/Global.Global_C|GetMouseFulfilled (Utilities|Array|Get(acopy) _outactors_3)) 20)
            (Default|CallMouseWon (Utilities|Array|Get(acopy) _outactors_3))))))))

(event Input|AxisEvents|InputAxisMoveForward
  (params (AxisValue :type Float%20%28single-precision%29))
  (bind _returnvalue (* AxisValue 4.0))
  (bind _mousecollider (Variables|Default|GetMouseCollider))
  (bind _returnvalue_2 (Math|Vector|GetForwardVector _mousecollider))
  (bind _returnvalue_3 (* _returnvalue_2 _returnvalue))
  ;[1 1 1] Movement Controls
  (if (Game|Player|IsInputKeyDown (Game|GetPlayerController 0) "W")
    (Utilities|Casting|CastToMouseBP (Game|Player|GetPlayerPawn 0))
    (Transformation|AddWorldOffset (Variables|Default|GetMouseCollider) _returnvalue_3 false false)
    (CallFunction|ROCLocation _returnvalue_3)))

(event Input|AxisEvents|InputAxisTurn
  (params (AxisValue :type Float%20%28single-precision%29))
  (bind _returnvalue (Transformation|GetActorRotation))
  (bind _returnvalue_2 (* AxisValue 3.0))
  (bind _returnvalue_3 (Math|Rotator|GetRotationXVector _returnvalue))
  (bind _returnvalue_4 (Math|Vector|RotateVectorAroundAxis _returnvalue_3 _returnvalue_2 "0, 0,1.000000"))
  (bind _returnvalue_5 (Math|Conversions|RotationFromXVector _returnvalue_4))
  ;[1 1 1] Movement Controls
  (if (Game|Player|IsInputKeyDown (Game|GetPlayerController 0) "A")
    (Utilities|Casting|CastToMouseBP (Game|Player|GetPlayerPawn 0) :!label _label)
    (Transformation|SetActorRotation _returnvalue_5)
    (CallFunction|ROCRotation _returnvalue_5)
    (elif (Game|Player|IsInputKeyDown (Game|GetPlayerController 0) "D")
      (goto _label))))

(fn ConstructionScript)