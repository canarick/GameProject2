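; Player-controlled waiter that carries dishes to tables and swats mice with a broom.
; Axis inputs offset the collider forward without sweep and rotate the actor.
; Tick polls Space to pick up a nearby plate or otherwise hold the broom, set it down destroying close mice, or serve the plate at a nearby table, clearing a matching order.
; Mesh and material swaps show what is held, and targets are found through GetAllActorsOfClass searches.
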(event EventBeginPlay)

(event Collision|EventActorBeginOverlap
  (params (OtherActor :type Actor%20Object%20Reference)))

(event EventTick
  (params (DeltaSeconds :type Float%20%28single-precision%29))
  (if (Game|Player|WasInputKeyJustPressed (Game|GetPlayerController 0) "SpaceBar")
    (if (Variables|Default|GetholdingBroom)
      ;[1 1 1] put down broom
      (bind _outactors (Actor|GetAllActorsOfClass "/Game/Blueprints/MouseBP.MouseBP_C"))
      (for _array_element _outactors
        (if (< (Transformation|GetDistanceTo _array_element) 6e+01)
          (Actor|DestroyActor _array_element)))
      (Variables|Default|SetholdingBroom false)
      (Rendering|Material|SetMaterial (Variables|Default|GetWaiterMesh) 0 "/Game/StarterContent/Materials/M_Basic_Wall.M_Basic_Wall")
      (elif (Variables|Default|GetholdingPlate)
        ;[1 1 1] put down plate on table
        (bind _outactors_2 (Actor|GetAllActorsOfClass "/Game/Blueprints/Table.Table_C"))
        (bind _array_element_2 (Utilities|Array|ForEachLoopwithBreak _outactors_2 :!label _label)
          (:LoopBody
            (if (Variables|/Game/Blueprints/Table.Table_C|GetWaiterCloseBy _array_element_2)
              (Game|SpawnActorfromClass "/Game/Blueprints/Plate.Plate_C" (Math|Transform|MakeTransform (+ (.location (Transformation|GetActorTransform _array_element_2)) "0,0.000000,100.000000") (.rotation (Transformation|GetActorTransform _array_element_2)) (.scale (Transformation|GetActorTransform _array_element_2))) "AlwaysSpawn" 0 (Variables|Default|GetholdingDish) true 0)
              (bind _outactors_3 (Actor|GetAllActorsOfClass "/Game/Blueprints/WaiterOrderBP.WaiterOrderBP_C"))
              (bind _array_element_3 (Utilities|Array|ForEachLoopwithBreak _outactors_3 :!label _label_2)
                (:LoopBody
                  (if (== (Variables|/Game/Blueprints/WaiterOrderBP.WaiterOrderBP_C|GetTable _array_element_3) (Variables|/Game/Blueprints/Table.Table_C|GetNumber _array_element_2))
                    (if (== (Variables|/Game/Blueprints/WaiterOrderBP.WaiterOrderBP_C|GetDish _array_element_3) (Variables|Default|GetholdingDish))
                      (Actor|DestroyActor _array_element_3)
                      (Default|CallRemoveOrder)
                      (goto _label_2 Break))))
                (:Completed
                  (Variables|Default|SetholdingPlate false)
                  (Components|StaticMesh|SetStaticMesh (Variables|Default|GetWaiterMesh) "/Game/Meshes/standing.standing")
                  (goto _label Break))))))
        (else
          ;[1 1 1] pick up plate
          (bind _outactors_4 (Actor|GetAllActorsOfClass "/Game/Blueprints/Plate.Plate_C"))
          (bind _array_element_4 (Utilities|Array|ForEachLoopwithBreak _outactors_4 :!label _label_3)
            (:LoopBody
              (if (< (Transformation|GetDistanceTo _array_element_4 self) 75.0)
                (Variables|Default|SetholdingDish (Variables|/Game/Blueprints/Plate.Plate_C|GetDish _array_element_4))
                (Actor|DestroyActor _array_element_4)
                (Variables|Default|SetholdingPlate true)
                (Development|PrintString "IsHoldingPlate")
                (Components|StaticMesh|SetStaticMesh (Variables|Default|GetWaiterMesh) "/Game/Meshes/holdPlateCombined.holdPlateCombined")
                (goto _label_3 Break)))
            (:Completed
              ;[1 1 1] hold broom
              (if (not (Variables|Default|GetholdingPlate))
                (Variables|Default|SetholdingBroom true)
                (Development|PrintString "is holding broom")
                (Rendering|Material|SetMaterial (Variables|Default|GetWaiterMesh) 0 "/Game/StarterContent/Materials/M_Metal_Gold.M_Metal_Gold")))))))))

(event Input|AxisEvents|InputAxisMoveForwardWaiter
  (params (AxisValue :type Float%20%28single-precision%29))
  (Transformation|AddWorldOffset (Variables|Default|GetWaiterCollider) (* (Math|Vector|GetForwardVector (Variables|Default|GetWaiterCollider)) (* AxisValue 3.0)) false false))

(event Input|AxisEvents|InputAxisTurnWaiter
  (params (AxisValue :type Float%20%28single-precision%29))
  (Transformation|SetActorRotation (Math|Conversions|RotationFromXVector (Math|Vector|RotateVectorAroundAxis (Math|Rotator|GetRotationXVector (Transformation|GetActorRotation)) (* AxisValue 2.0) "0, 0,1.000000"))))

(fn ConstructionScript)