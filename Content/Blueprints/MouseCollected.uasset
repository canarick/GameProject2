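; MouseCollected is an actor that mirrors a collected dish in the CollectedList of the MouseInGame HUD widget.
; On BeginPlay it creates a MouseCollectedUI entry from its Dish and Drop values and adds it to that list.
; When destroyed, it removes the first entry flagged Drop, which is not matched to the actor itself, then passes the flag to the entry at the top of the list.
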(event EventBeginPlay
  (bind _returnvalue (UserInterface|CreateWidget "/Game/Blueprints/Widget/MouseCollectedUI.MouseCollectedUI_C" 0 (Variables|Default|GetDish) (Variables|Default|GetDrop)))
  (bind _foundwidgets (Widget|GetAllWidgetsOfClass "/Game/Blueprints/Widget/MouseInGame.MouseInGame_C" true))
  (Widget|Panel|AddChild (Variables|/Game/Blueprints/Widget/MouseInGame.MouseInGame_C|GetCollectedList (Utilities|Array|Get(acopy) _foundwidgets)) _returnvalue))

(event Collision|EventActorBeginOverlap
  (params (OtherActor :type Actor%20Object%20Reference)))

(event EventTick
  (params (DeltaSeconds :type Float%20%28single-precision%29)))

(event EventDestroyed
  (bind _foundwidgets (Widget|GetAllWidgetsOfClass "/Game/Blueprints/Widget/MouseInGame.MouseInGame_C" true))
  (bind (_array_element _array_index) (Utilities|Array|ForEachLoopwithBreak (Class|PanelWidget|GetAllChildren (Variables|/Game/Blueprints/Widget/MouseInGame.MouseInGame_C|GetCollectedList (Utilities|Array|Get(acopy) _foundwidgets))) :!label _label)
    (:LoopBody
      (bind _asmouse_collected_ui (Utilities|Casting|CastToMouseCollectedUI _array_element))
      (if (Variables|/Game/Blueprints/Widget/MouseCollectedUI.MouseCollectedUI_C|GetDrop _asmouse_collected_ui)
        (Class|PanelWidget|RemoveChildat (Variables|/Game/Blueprints/Widget/MouseInGame.MouseInGame_C|GetCollectedList (Utilities|Array|Get(acopy) _foundwidgets)) _array_index)
        (goto _label Break)))
    (:Completed
      (bind _asmouse_collected_ui_2 (Utilities|Casting|CastToMouseCollectedUI (Class|PanelWidget|GetChildat (Variables|/Game/Blueprints/Widget/MouseInGame.MouseInGame_C|GetCollectedList (Utilities|Array|Get(acopy) _foundwidgets)))))
      (Variables|/Game/Blueprints/Widget/MouseCollectedUI.MouseCollectedUI_C|SetDrop _asmouse_collected_ui_2 true))))

(fn ConstructionScript)